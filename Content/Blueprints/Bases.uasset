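; Bases Blueprint that serves as a scratch catalogue of common nodes, apparently for reference, with little working game logic.
; On BeginPlay it adds the HUD widget and enables Game-and-UI input with a visible cursor, while Tick prints the frame delta.
; Everything else is disconnected example nodes under Spanish headings covering variables, flow control, operations, UI, movement, traces, audio and particles.
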(event `self.ReceiveBeginPlay`
  (bind _returnvalue (`GameplayStatics.GetPlayerController` 0))
  (bind _returnvalue_2 (`|CreateWidget` "/Game/Blueprints/HUD.HUD_C"))
  (`UserWidget.AddToViewport` _returnvalue_2 0)
  (`WidgetBlueprintLibrary.SetInputMode_GameAndUIEx` _returnvalue _returnvalue_2)
  (set `PlayerController.bShowMouseCursor` true _returnvalue))

(event `CustomEvent_0`
  ;[0.1413 0.3125 0] Flow control
)

(event `self.ReceiveTick`
  (params (DeltaSeconds :type "Float (single-precision)"))
  (`KismetSystemLibrary.PrintString` (`KismetStringLibrary.Conv_DoubleToString` DeltaSeconds)))

(event `Key|Tab`
  (params (Key :type "Key Structure")))

(event `InputAction|Jump`
  (params (Key :type "Key Structure")))

(fn `UserConstructionScript`)